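; Behavior Tree task that finds an enemy Shooter for the AI robot and stores it in the Enemy blackboard key.
; On execute, it runs a huge-radius multi sphere trace on the Camera channel around the RobotController's shooter.
; Hit Shooters are filtered with IsEnemy, with no break after a match.
; The task reports success even when no enemy is found.
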(event EventReceiveExecute
  (params (OwnerActor :type Actor%20Object%20Reference))
  (bind _asrobot_controller (Utilities|Casting|CastToRobotController OwnerActor))
  (bind (_outhits _returnvalue) (Collision|MultiSphereTraceByChannel (Transformation|GetActorLocation (Default|GetRobotShooter _asrobot_controller)) (+ (Transformation|GetActorLocation (Default|GetRobotShooter _asrobot_controller)) "0, 0,10.000000") 6e+05 "TraceTypeQuery2" false 0 "None"))
  (if _returnvalue
    (for _array_element _outhits
      (bind _asshooter (Utilities|Casting|CastToShooter (.HitActor (Collision|BreakHitResult _array_element))))
      (if (Default|IsEnemy _asshooter (Default|GetRobotShooter _asrobot_controller))
        (Class|BTFunctionLibrary|SetBlackboardValueasObject (Utilities|Struct|MakeBlackboardKeySelector (Utilities|Array|MakeArray 0) "Enemy") _asshooter)
        (AI|BehaviorTree|FinishExecute true))))
  (AI|BehaviorTree|FinishExecute true))