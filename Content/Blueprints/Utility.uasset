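; Utility function library that supplies random character names and team colors for a shooter.
; GetRandomName joins a random family name and a random given name from two arrays, family name first with no separator.
; GetSideColor compares a given side with that of the FppShooter pawn of player 0, returning blue for a match and red otherwise, so colors are relative to that player.
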(fn GetRandomName
  (return (Utilities|String|Append (Utilities|Array|Get(acopy) (LocalVariables|GetFamilyNameArray) (Math|Random|RandomIntegerinRange 0 (- (Utilities|Array|Length (LocalVariables|GetFamilyNameArray)) 1))) (Utilities|Array|Get(acopy) (LocalVariables|GetGivenNameArray) (Math|Random|RandomIntegerinRange 0 (- (Utilities|Array|Length (LocalVariables|GetGivenNameArray)) 1))))))

(fn GetSideColor
  (params (Side :type Integer))
  (bind _asfpp_shooter (Utilities|Casting|CastToFppShooter (Game|Player|GetPlayerPawn (LocalVariables|Get__WorldContext))))
  (return (select (== Side (Variables|/Game/Blueprints/Shooter.Shooter_C|GetSide _asfpp_shooter)) (Utilities|Struct|MakeLinearColor 0.0 0.0 1.0 1.0) (Utilities|Struct|MakeLinearColor 1.0 0.0 0.0 1.0))))