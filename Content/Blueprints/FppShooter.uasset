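; First-person shooter character that moves, looks, fires, reloads and cycles between a Rifle and a Launcher created at BeginPlay.
; Firing and reloading are delegated to the current gun actor, with shot origin and direction exposed from the camera and control rotation.
; Switching toggles gun visibility, plays an equip montage and uses a timestamp to block firing and re-switching during equip.
; Death pulls the camera back and ragdolls a third-person mesh; keys open rank and main UI widgets.
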(event EventBeginPlay
  (CallFunction|CreateGun "/Game/Blueprints/Rifle.Rifle_C")
  (CallFunction|CreateGun "/Game/Blueprints/Launcher.Launcher_C")
  (Variables|Default|SetCurrentIndex 1)
  (Rendering|SetActorHiddenInGame (CallFunction|GetCurrentGun) false))

(event EventOnDie
  (bind _mesh (Variables|Character|GetMesh))
  (Transformation|AddLocalOffset (Variables|Default|GetCamera) "-600.000000, 0, 0" false false)
  (Class|SkinnedMeshComponent|SetSkeletalMesh _mesh "/Game/Assets/Characters/Models/HeroTPP.HeroTPP" true)
  (Physics|SetSimulatePhysics _mesh true)
  (Collision|SetCollisionEnabled _mesh "QueryAndPhysics"))

(event Input|ActionEvents|InputActionFire
  (params (Key :type Key%20Structure :default "AnyKey"))
  (:Pressed
    (CallFunction|StartFire))
  (:Released
    (CallFunction|EndFire)))

(event Input|ActionEvents|InputActionEquip
  (params (Key :type Key%20Structure :default "AnyKey"))
  (:Pressed
    (CallFunction|SwitchWeapon)))

(event Input|ActionEvents|InputActionReload
  (params (Key :type Key%20Structure :default "AnyKey"))
  (:Pressed
    (CallFunction|Reload)))

(event Input|AxisEvents|InputAxisMoveForward
  (params (AxisValue :type Float%20%28single-precision%29))
  (Pawn|Input|AddMovementInput (Math|Vector|GetForwardVector (Pawn|GetControlRotation :!class /Script/Engine.Pawn)) AxisValue false))

(event Input|AxisEvents|InputAxisTurn
  (params (AxisValue :type Float%20%28single-precision%29))
  (Pawn|Input|AddControllerYawInput AxisValue))

(event Input|AxisEvents|InputAxisLookUp
  (params (AxisValue :type Float%20%28single-precision%29))
  (Pawn|Input|AddControllerPitchInput AxisValue))

(event Input|AxisEvents|InputAxisMoveRight
  (params (AxisValue :type Float%20%28single-precision%29))
  (Pawn|Input|AddMovementInput (Math|Vector|GetRightVector (Pawn|GetControlRotation :!class /Script/Engine.Pawn)) AxisValue false))

(event Input|KeyboardEvents|Tab
  (params (Key :type Key%20Structure :default "AnyKey"))
  (:Pressed
    (bind _returnvalue (UserInterface|CreateWidget "/Game/Blueprints/UI/RankPanel.RankPanel_C"))
    (bind _output_get (Variables|Default|SetRankPanel _returnvalue))
    (UserInterface|Viewport|AddtoViewport _output_get 0))
  (:Released
    (Widget|RemovefromParent (Variables|Default|GetRankPanel))))

(event Input|KeyboardEvents|B
  (params (Key :type Key%20Structure :default "AnyKey"))
  (:Pressed
    (bind _returnvalue (UserInterface|CreateWidget "/Game/Blueprints/UI/Main_UI.Main_UI_C"))
    (UserInterface|Viewport|AddtoViewport _returnvalue 0)))

(fn ConstructionScript
  (|CallParentFunction))

(fn StartFire
  (if (not (CallFunction|IsinEquip))
    (Default|StartFire (CallFunction|GetCurrentGun))))

(fn EndFire
  (Default|EndFire (CallFunction|GetCurrentGun)))

(fn SwitchWeapon
  (bind _gun (CallFunction|GetCurrentGun))
  (if (not (CallFunction|IsinEquip))
    (Default|EndFire _gun)
    (Rendering|SetActorHiddenInGame _gun true)
    (Variables|Default|SetCurrentIndex (Math|Integer|%(Integer) (+ (Variables|Default|GetCurrentIndex) 1) (Utilities|Array|Length (Variables|Default|GetGuns))))
    (Rendering|SetActorHiddenInGame (CallFunction|GetCurrentGun) false)
    (Animation|PlayAnimMontage "/Game/Blueprints/FppEquip_Montage.FppEquip_Montage" 1.0 "None")
    (Variables|Default|SetEquipTime (Utilities|Time|GetTimeSeconds))
    (Default|CallChangeGunDispatcher)))

(fn IsinEquip
  (return (< (- (Utilities|Time|GetTimeSeconds) (Variables|Default|GetEquipTime)) (Variables|Default|GetEquipTimeLength))))

(fn GetShootLocation
  (return (Transformation|GetWorldLocation (Variables|Default|GetCamera))))

(fn GetShootDirection
  (return (Math|Vector|GetForwardVector (Pawn|GetControlRotation :!class /Script/Engine.Pawn))))

(fn Reload
  (Default|PlayReload (CallFunction|GetCurrentGun)))