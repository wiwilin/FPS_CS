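; Launcher weapon actor that fires a single projectile per trigger press for its owning character.
; StartFire calls ShootOnce, which uses the fire animation length as a cooldown, spends one round, spawns a Bullet from the muzzle along the owner's control rotation and plays the fire montage.
; PlayReload only plays the reload montage on the owner, and GetIcon returns the launcher's icon.
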(event EventBeginPlay)

(event Collision|EventActorBeginOverlap
  (params (OtherActor :type Actor%20Object%20Reference)))

(event EventStartFire
  (CallFunction|ShootOnce))

(event EventShootOnce
  (if (>= (- (Utilities|Time|GetTimeSeconds) (Variables|Default|GetLastShootTime)) (Variables|Default|GetShootAnimTimeLength))
    (if (> (Variables|Default|GetBulletNum) 0)
      (Math|Integer|DecrementInt (Variables|Default|GetBulletNum)
        (:%20%20
          (Game|SpawnActorfromClass "/Game/Blueprints/Bullet.Bullet_C" (Math|Transform|MakeTransform (Transformation|GetWorldLocation (Variables|Default|GetMuzzle)) (Pawn|GetControlRotation (Variables|Default|GetGunOwner) :!class /Script/Engine.Pawn) "1,1,1") "Undefined" 0 (Variables|Default|GetGunOwner) 0)
          (Animation|PlayAnimMontage (Variables|Default|GetGunOwner) "/Game/Blueprints/FppLauncherFire_Montage.FppLauncherFire_Montage" 1.0 "None")
          (Variables|Default|SetLastShootTime (Utilities|Time|GetTimeSeconds)))))))

(event EventPlayReload
  (Animation|PlayAnimMontage (Variables|Default|GetGunOwner) "/Game/Blueprints/LauncherReload_Montage.LauncherReload_Montage" 1.0 "None"))

(event EventTick
  (params (DeltaSeconds :type Float%20%28single-precision%29)))

(fn ConstructionScript
  (|CallParentFunction))

(fn GetIcon
  (return "/Game/Assets/UI/launcher_icon.launcher_icon"))