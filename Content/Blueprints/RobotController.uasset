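; RobotController is an AI controller that runs the Robot_BT behavior tree with the Robot_BB blackboard.
; On BeginPlay it stores itself under the blackboard's Gun key.
; Perception updates set CanSeeEnemy from sensing success when the actor matches the Enemy key, which is not assigned here.
; An unconnected leftover chain would make the RobotShooter pawn always shoot and repeatedly move toward the player.
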(event OnTargetPerceptionUpdated(AIPerception)
  (params (Actor :type Actor%20Object%20Reference) (Stimulus :type AI%20Stimulus%20Structure))
  (bind _returnvalue (AI|GetBlackboard 0))
  (if (== Actor (AI|Components|Blackboard|GetValueasObject _returnvalue (Utilities|Name|MakeLiteralName "Enemy")))
    (AI|Components|Blackboard|SetValueasBool _returnvalue (Utilities|Name|MakeLiteralName "CanSeeEnemy") (.bSuccessfullySensed (Utilities|Struct|BreakAIStimulus Stimulus)))))

(event EventBeginPlay
  (Class|AIController|UseBlackboard "/Game/Blueprints/AI/Robot_BB.Robot_BB")
  (AI|RunBehaviorTree "/Game/Blueprints/AI/Robot_BT.Robot_BT")
  (AI|Components|Blackboard|SetValueasObject (AI|GetBlackboard 0) (Utilities|Name|MakeLiteralName "Gun") self))

(fn ConstructionScript)

(fn GetRobotShooter
  (bind _asrobot_shooter (Utilities|Casting|CastToRobotShooter (Pawn|GetControlledPawn)))
  (return _asrobot_shooter))