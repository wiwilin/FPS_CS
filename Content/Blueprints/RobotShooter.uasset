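; RobotShooter is an AI-driven robot character that fights with a rifle, which it creates and makes visible on BeginPlay.
; AlwaysShoot starts continuous fire on the current gun, while ShootEnemy fires a single shot.
; Aim runs from the actor's location toward the Shooter stored under the AI blackboard's "Enemy" key, or is zero without a valid AI controller.
; OnDeathAnimPlayOver destroys the actor.
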(event EventBeginPlay
  (CallFunction|CreateGun "/Game/Blueprints/Rifle.Rifle_C")
  (Variables|Default|SetCurrentIndex 0)
  (Rendering|SetActorHiddenInGame (CallFunction|GetCurrentGun) false))

(event Collision|EventActorBeginOverlap
  (params (OtherActor :type Actor%20Object%20Reference)))

(event EventTick
  (params (DeltaSeconds :type Float%20%28single-precision%29)))

(fn ConstructionScript
  (|CallParentFunction))

(fn OnDeathAnimPlayOver
  (Actor|DestroyActor))

(fn GetShootLocation
  (return (Transformation|GetActorLocation)))

(fn AlwaysShoot
  (Default|StartFire (CallFunction|GetCurrentGun)))

(fn ShootEnemy
  (Default|ShootOnce (CallFunction|GetCurrentGun)))

(fn GetShootDirection
  (bind _self self)
  (bind _returnvalue (AI|GetAIController _self))
  (Utilities|IsValid _returnvalue
    (:Is%20Valid
      (bind _asshooter (Utilities|Casting|CastToShooter (AI|Components|Blackboard|GetValueasObject (AI|GetBlackboard _returnvalue) (Utilities|Name|MakeLiteralName "Enemy"))))
      (return (- (Transformation|GetActorLocation _asshooter) (Transformation|GetActorLocation))))
    (:Is%20Not%20Valid
      (return "0, 0, 0"))))