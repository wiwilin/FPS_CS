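; Base combatant pawn with health, a random name, a team side and a set of owned guns.
; CreateGun spawns hidden guns on the right-hand socket, and destroying the shooter destroys them.
; Lethal damage stops all guns firing, reports the kill to ShooterGameMode's dispatcher and schedules a delayed controller detach.
; OnDie and the shoot location and direction getters are placeholders, apparently for child classes to override.
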(event EventBeginPlay)

(event Collision|EventActorBeginOverlap
  (params (OtherActor :type Actor%20Object%20Reference)))

(event EventTick
  (params (DeltaSeconds :type Float%20%28single-precision%29)))

(event EventDestroyed
  (for _array_element (Variables|Default|GetGuns)
    (Actor|DestroyActor _array_element)))

(fn ConstructionScript
  (Variables|Default|SetHealth (Variables|Default|GetMaxHealth))
  (Variables|Default|SetName (CallFunction|GetRandomName)))

(fn TakeDamage
  (params (Damage :type Float%20%28single-precision%29) (Enemy :type Shooter%20Object%20Reference))
  (if (not (CallFunction|IsDead))
    (bind _output_get (Variables|Default|SetHealth (- (Variables|Default|GetHealth) Damage)))
    (Development|PrintString (Utilities|String|ToString(Float) _output_get))
    (if (CallFunction|IsDead)
      (CallFunction|Die Enemy))))

(fn IsDead
  (return (<= (Variables|Default|GetHealth) 0.0)))

(fn GetShootLocation
  (return "0, 0, 0"))

(fn CreateGun
  (params (GunClass :type Gun%20Class%20Reference))
  (bind _returnvalue (Game|SpawnActorfromClass GunClass (Math|Transform|MakeTransform "0, 0, 0" "0, 0, 0" "1,1,1") "Undefined" 0 0))
  (Transformation|AttachComponentToComponent _returnvalue (Variables|Character|GetMesh) "RightWeapon" "SnapToTarget" "SnapToTarget" "SnapToTarget" true)
  (Variables|/Game/Blueprints/Gun.Gun_C|SetGunOwner _returnvalue self)
  (Utilities|Array|Add (Variables|Default|GetGuns) _returnvalue)
  (Rendering|SetActorHiddenInGame _returnvalue true))

(fn GetCurrentGun
  (return (Utilities|Array|Get(acopy) (Variables|Default|GetGuns) (Variables|Default|GetCurrentIndex))))

(fn OnDie)

(fn Die
  (params (Enemy :type Shooter%20Object%20Reference))
  (for _array_element (Variables|Default|GetGuns)
    (Default|EndFire _array_element))
  (bind _asshooter_game_mode (Utilities|Casting|CastToShooterGameMode (Game|GetGameMode)))
  (Default|CallKillDispatcher _asshooter_game_mode (Variables|Shooter_C|GetName Enemy) (Variables|Default|GetName) (Variables|Shooter_C|GetSide Enemy) (Variables|Default|GetSide) (Default|GetIcon (CallFunction|GetCurrentGun Enemy)))
  (CallFunction|OnDie)
  (Utilities|Time|SetTimerbyFunctionName 0 "DetachFromControllerPendingDestroy" 2e+01))

(fn GetShootDirection
  (return "0, 0, 0"))

(fn IsEnemy
  (params (Shooter :type Shooter%20Object%20Reference))
  (return (!= (Variables|Shooter_C|GetSide Shooter) (Variables|Default|GetSide))))