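; Rifle is an automatic hitscan weapon for a Shooter owner, with its own icon and reload montage.
; StartFire plays the fire montage and muzzle flash, then runs ShootOnce immediately and on a looping timer until EndFire.
; ShootOnce spends a bullet and line-traces on Camera with persistent debug lines, damaging enemy Shooters, or calls EndFire when empty.
; PlayReload only plays animation, and a disconnected multi-trace variant remains unused.
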(event EventBeginPlay)

(event Collision|EventActorBeginOverlap
  (params (OtherActor :type Actor%20Object%20Reference)))

(event EventStartFire
  (Utilities|FlowControl|Sequence
    (:then_0
      (Animation|PlayAnimMontage (Variables|Default|GetGunOwner) "/Game/Blueprints/FppRifleFire_Montage.FppRifleFire_Montage" 1.0 "None")
      (bind _returnvalue (Effects|SpawnEmitterAttached "/Game/Assets/Effects/ParticleSystems/Weapons/AssaultRifle/Muzzle/P_AssaultRifle_MF.P_AssaultRifle_MF" (Variables|Default|GetMuzzle) "None"))
      (Variables|Default|SetFireEffects _returnvalue))
    (:then_1
      (CallFunction|ShootOnce)
      (Utilities|Time|SetTimerbyFunctionName 0 "ShootOnce" 0.2 true))
    (:then_2
      (Variables|Default|SetIsInFire true))))

(event EventEndFire
  (if (Variables|Default|GetIsInFire)
    (Utilities|FlowControl|Sequence
      (:then_0
        (Animation|StopAnimMontage (Variables|Default|GetGunOwner) "/Game/Blueprints/FppRifleFire_Montage.FppRifleFire_Montage")
        (Components|DestroyComponent (Variables|Default|GetFireEffects)))
      (:then_1
        (Utilities|Time|ClearTimerbyFunctionName 0 "ShootOnce"))
      (:then_2
        (Variables|Default|SetIsInFire false)))))

(event EventPlayReload
  (Animation|PlayAnimMontage (Variables|Default|GetGunOwner) "/Game/Blueprints/RifleReload_Montage.RifleReload_Montage" 1.0 "None"))

(event EventTick
  (params (DeltaSeconds :type Float%20%28single-precision%29)))

(event EventShootOnce
  (bind _gunowner (Variables|Default|GetGunOwner))
  (bind _location (Default|GetShootLocation _gunowner))
  (if (> (Variables|Default|GetBulletNum) 0)
    (Math|Integer|DecrementInt (Variables|Default|GetBulletNum)
      (:%20%20
        (bind (_outhit _returnvalue) (Collision|LineTraceByChannel _location (+ (* (Math|Vector|Normalize (Default|GetShootDirection (Variables|Default|GetGunOwner))) 1.5e+03) _location) "TraceTypeQuery2" false (Utilities|Array|MakeArray (Variables|Default|GetGunOwner)) "Persistent"))
        (if _returnvalue
          (bind _asshooter (Utilities|Casting|CastToShooter (.HitActor (Collision|BreakHitResult _outhit))))
          (if (Default|IsEnemy _asshooter (Variables|Default|GetGunOwner))
            (Default|TakeDamage _asshooter 2e+01 (Variables|Default|GetGunOwner))))))
    (else
      (CallFunction|EndFire))))

(fn ConstructionScript
  (|CallParentFunction))

(fn GetIcon
  (return "/Game/Assets/UI/rifle_icon.rifle_icon"))